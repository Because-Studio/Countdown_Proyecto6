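; Interactable actor that reacts when a magic object overlaps it.
; On overlap, its BPCMagicInteractuable component checks the other actor, and a passing check calls ObjectAction and prints a confirmation.
; ObjectAction scales the static mesh up uniformly.
; The construction script assigns the mesh from the NewMesh variable.
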(event `self.ReceiveActorBeginOverlap`
  (params (OtherActor :type "Actor Object Reference"))
  ;[0.002066 1 0] ACTOR BEGIN OVERLAP
  (bind (_condition_ _hitbymagic_) (`/Game/Blueprints/BPComponents/BPC_MagicInteractuable.checkMagic` (`self.BPC_MagicInteractuable`) OtherActor))
  (if _condition_
    (`self.ObjectAction`)
    (`KismetSystemLibrary.PrintString` "Interaction DONE!")
    (elif _hitbymagic_
      _)))

(event `ObjectAction`
  ;[1 0.06317 0.9242] CustomEvent
  (`SceneComponent.SetWorldScale3D` (`self.StaticMesh`) (5.0 5.0 5.0)))

(fn `UserConstructionScript`
  (`StaticMeshComponent.SetStaticMesh` (`self.StaticMesh`) (`self.New Mesh`)))