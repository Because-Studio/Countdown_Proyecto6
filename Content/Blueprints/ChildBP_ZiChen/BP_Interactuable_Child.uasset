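; Interactable child Blueprint that unlocks a key receiver in the level when its action fires while the linked key's light is active.
; On BeginPlay it caches the BP_Key_SameLevel_Child and BP_Receiver_Child actors found by class lookup.
; ObjectAction checks the key's LightActived flag, then turns the receiver's cube gold and sets its KeyCanPick flag.
; The overlap event only forwards to the parent.
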(event `self.ReceiveBeginPlay`
  (bind _returnvalue (`GameplayStatics.GetActorOfClass` "/Game/Blueprints/ChildBP_ZiChen/BP_Key_SameLevel_Child.BP_Key_SameLevel_Child_C"))
  (set `self.Light` _returnvalue)
  (bind _returnvalue_2 (`GameplayStatics.GetActorOfClass` "/Game/Blueprints/ChildBP_ZiChen/BP_Receiver_Child.BP_Receiver_Child_C"))
  (set `self.keyReceve` _returnvalue_2))

(event `self.ReceiveActorBeginOverlap`
  (params (OtherActor :type "Actor Object Reference"))
  ;[1 1 1] Sobreesbe su Coll
  (`parent.ReceiveActorBeginOverlap` OtherActor))

(event `self.ObjectAction`
  (bind _keyreceve (`self.keyReceve`))
  (if (`/Game/Blueprints/ChildBP_ZiChen/BP_Key_SameLevel_Child.lightActived?` (`self.Light`))
    (`PrimitiveComponent.SetMaterial` (`/Game/Blueprints/BP_Receiver.Cube` _keyreceve) 0 "/Game/Fantastic_Village_Pack/materials/MI_gold.MI_gold")
    (set `/Game/Blueprints/ChildBP_ZiChen/BP_Receiver_Child.keyCanPick?` true _keyreceve)))

(fn `UserConstructionScript`)