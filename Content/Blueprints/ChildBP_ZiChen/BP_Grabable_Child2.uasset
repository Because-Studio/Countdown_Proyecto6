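; BP_Grabable_Child2 is a child grabbable actor that pairs with a BP_Grabable_Child found in the level at BeginPlay.
; When an overlapping actor passes the BPCMagicInteractuable magic check and either of two object-in-location flags is set, it turns its GrabZone material red.
; It then increments an index counter and tells the paired grabbable to check that index.
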(event `self.ReceiveBeginPlay`
  (bind _returnvalue (`GameplayStatics.GetActorOfClass` "/Game/Blueprints/ChildBP_ZiChen/BP_Grabable_Child.BP_Grabable_Child_C"))
  (set `self.grabable1` _returnvalue))

(event `self.ReceiveActorBeginOverlap`
  (params (OtherActor :type "Actor Object Reference"))
  (`|ExecutionSequence`
    (:`then_0`
      (bind _condition_ (`/Game/Blueprints/BPComponents/BPC_MagicInteractuable.checkMagic` (`self.BPC_MagicInteractuable`) OtherActor))
      (if (and _condition_ (or (`self.object1_InLocation?`) (`self.object2_InLocarion?`)))
        (`PrimitiveComponent.SetMaterial` (`self.grabZone`) 0 "/Game/Material/M_Red.M_Red")
        (`/Engine/EditorBlueprintResources/StandardMacros.IncrementInt` (`self.Index_Control`)
          (:`  `
            (`/Game/Blueprints/ChildBP_ZiChen/BP_Grabable_Child.CE_CheckIndex` (`self.grabable1`))))))))

(fn `UserConstructionScript`
  (`parent.UserConstructionScript`))