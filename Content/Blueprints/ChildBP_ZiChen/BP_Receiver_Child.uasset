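; BP_Receiver_Child is a child receiver Blueprint that moves its Cube to a marker actor's location when it receives a matching ID message.
; BeginPlay caches the BP_Empty_MarkLocation actor found through GetActorOfClass.
; The ID event passes the incoming ID and its own to ReceiveMessageWithID, and a match triggers a custom event that teleports the Cube to the marker without sweep.
; A gold material swap on the Cube is left unconnected.
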(event `self.ReceiveTick`
  (params (DeltaSeconds :type "Float (single-precision)")))

(event `self.ReceiveBeginPlay`
  (bind _returnvalue (`GameplayStatics.GetActorOfClass` "/Game/Blueprints/ChildBP_ZiChen/BP_Empty_MarkLocation.BP_Empty_MarkLocation_C"))
  (set `self.Actor_MarkLocation` _returnvalue))

(event `/Game/Blueprints/Interfaces/BPI_EventReceiver.ReceiveEvent`
  (params (ID :type Integer))
  (bind _match_ (`/Game/Blueprints/Function/BPF_MessageWithID.ReceiveMessageWithID` ID (`self.ReceveID`)))
  (if _match_
    (`self.CE_SetLoc`)))

(event `CE_SetLoc`
  (`SceneComponent.K2_SetWorldLocation` (`self.Cube`) (`self.K2_GetActorLocation` (`self.Actor_MarkLocation`)) false true))

(fn `UserConstructionScript`
  (`parent.UserConstructionScript`))