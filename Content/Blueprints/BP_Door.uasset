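; BP_Door is a sliding door that the player opens with the Interact input once KeyDestroyed is true.
; A Box overlap enables and disables the door's input for the cached BP_Player, limiting interaction to that volume.
; A successful press plays a sound and runs a timeline that drives the Cube's relative Y position, with no reverse path.
; Otherwise a different sound plays; KeyDestroyed is only read here, never set.
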(event `self.ReceiveBeginPlay`
  (bind _asbp_player (cast `/Game/Player/BP_Player` (`GameplayStatics.GetPlayerCharacter` 0)))
  (set `self.BP Player` _asbp_player))

(event `InputAction|Interact`
  (params (Key :type "Key Structure"))
  (bind _cube (`self.Cube`))
  (bind (_relativelocation_x _relativelocation_y _relativelocation_z) (`KismetMathLibrary.BreakVector` (`SceneComponent.RelativeLocation` _cube)))
  (:`Pressed`
    (if (`self.keyDestroyed?`)
      (`GameplayStatics.PlaySound2D` "/Game/Sounds/Dockable_Window_Drop.Dockable_Window_Drop" 1.0 1.0 0.0 null null)
      (bind (_direction _trans) (`Timeline|Timeline_0`)
        (:`Update`
          (`SceneComponent.K2_SetRelativeLocation` _cube (`KismetMathLibrary.MakeVector` _relativelocation_x _trans _relativelocation_z) false false)))
      (else
        (`GameplayStatics.PlaySound2D` "/Game/Sounds/EndPlayInEditor.EndPlayInEditor" 1.0 1.0 0.0 null null)))))

(event `self.Box.OnComponentBeginOverlap`
  (params (OverlappedComponent :type "PrimitiveComponent Object Reference") (OtherActor :type "Actor Object Reference") (OtherComp :type "PrimitiveComponent Object Reference") (OtherBodyIndex :type Integer) (bFromSweep :type Boolean) (SweepResult :type "HitResult Structure (by ref)"))
  (if (== OtherActor (`self.BP Player`))
    (`self.EnableInput` (`GameplayStatics.GetPlayerController` 0))))

(event `self.Box.OnComponentEndOverlap`
  (params (OverlappedComponent :type "PrimitiveComponent Object Reference") (OtherActor :type "Actor Object Reference") (OtherComp :type "PrimitiveComponent Object Reference") (OtherBodyIndex :type Integer))
  (if (== OtherActor (`self.BP Player`))
    (`self.DisableInput` (`GameplayStatics.GetPlayerController` 0))))

(fn `UserConstructionScript`)