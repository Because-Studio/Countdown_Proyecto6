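; BPC_TalkableNPC is an actor component that lets the owning NPC hold a conversation using its assigned DialogueTree.
; On BeginPlay it casts the owner's AI controller to NPC_AI and copies DialogueTree into that controller.
; StartDialogue assigns the tree again, then delegates to the controller's StartDialogue.
; Both paths do nothing if the controller is not an NPC_AI.
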(event `self.ReceiveBeginPlay`
  (bind _asnpc_ai (cast `/Game/Blueprints/NPC_AI` (`AIBlueprintHelperLibrary.GetAIController` (`self.GetOwner`))))
  (set `/Game/Blueprints/NPC_AI.DialogTree` (`self.DialogueTree`) _asnpc_ai))

(fn `StartDialogue`
  (bind _asnpc_ai (cast `/Game/Blueprints/NPC_AI` (`AIBlueprintHelperLibrary.GetAIController` (`self.GetOwner`))))
  (set `/Game/Blueprints/NPC_AI.DialogTree` (`self.DialogueTree`) _asnpc_ai)
  (`/Game/Blueprints/NPC_AI.StartDialogue` _asnpc_ai))