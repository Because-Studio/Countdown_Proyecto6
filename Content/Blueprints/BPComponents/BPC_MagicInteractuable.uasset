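; Actor component that decides whether a magic spell hitting an interactable object meets that object's requirements.
; CheckMagic compares the impact object's class against nine fire, ice and lightning spell classes to get an element and level.
; CheckMagicPart2 tests these against per-element flags, where each level flag accepts that level or higher and AllMagic accepts any spell.
; It returns whether the condition passes and whether magic hit at all.
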(event `self.ReceiveBeginPlay`)

(fn `checkMagic`
  (params (impactObject :type "Actor Object Reference"))
  (returns (`Condition?` :type Boolean) (`HitByMagic?` :type Boolean))
  (locals (classImpactObject :type "Actor Class Reference"))
  (set `local.classImpactObject` (`GameplayStatics.GetObjectClass` impactObject))
  (if (== (`local.classImpactObject`) (`self.As BP FireLvl1`))
    (bind (_condition _hitbymagic) (`self.checkMagicPart2` true 1 1))
    (return _condition _hitbymagic)
    (elif (== (`local.classImpactObject`) (`self.As BP FireLvl2`))
      (bind (_condition_2 _hitbymagic_2) (`self.checkMagicPart2` true 1 2))
      (return _condition_2 _hitbymagic_2)
      (elif (== (`local.classImpactObject`) (`self.As BP FireLvl3`))
        (bind (_condition_3 _hitbymagic_3) (`self.checkMagicPart2` true 1 3))
        (return _condition_3 _hitbymagic_3)
        (elif (== (`local.classImpactObject`) (`self.As BP  IceLvl1`))
          (bind (_condition_4 _hitbymagic_4) (`self.checkMagicPart2` true 2 1))
          (return _condition_4 _hitbymagic_4)
          (elif (== (`local.classImpactObject`) (`self.As BP IceLvl2`))
            (bind (_condition_5 _hitbymagic_5) (`self.checkMagicPart2` true 2 2))
            (return _condition_5 _hitbymagic_5)
            (elif (== (`local.classImpactObject`) (`self.As BP IceLvl3`))
              (bind (_condition_6 _hitbymagic_6) (`self.checkMagicPart2` true 2 3))
              (return _condition_6 _hitbymagic_6)
              (elif (== (`local.classImpactObject`) (`self.As BP LightningLvl1`))
                (bind (_condition_7 _hitbymagic_7) (`self.checkMagicPart2` true 3 1))
                (return _condition_7 _hitbymagic_7)
                (elif (== (`local.classImpactObject`) (`self.As BP LightningLvl2`))
                  (bind (_condition_8 _hitbymagic_8) (`self.checkMagicPart2` true 3 2))
                  (return _condition_8 _hitbymagic_8)
                  (elif (== (`local.classImpactObject`) (`self.As BP LightningLvl3`))
                    (bind (_condition_9 _hitbymagic_9) (`self.checkMagicPart2` true 3 3))
                    (return _condition_9 _hitbymagic_9)
                    (else
                      (bind (_condition_10 _hitbymagic_10) (`self.checkMagicPart2` false))
                      (return _condition_10 _hitbymagic_10))))))))))))

(fn `checkMagicPart2`
  (params (`IsMagic?` :type Boolean) (MagicType :type Integer) (MagicLvl :type Integer))
  (returns (Condition :type Boolean) (HitByMagic :type Boolean))
  (locals (MagicType_0 :type Integer) (MagicLvl_0 :type Integer) (isMagic :type Boolean))
  (bind _output_get (set `local.isMagic` `IsMagic?`))
  (if _output_get
    (set `local.MagicType_0` MagicType)
    (set `local.MagicLvl_0` MagicLvl)
    (if (`self.AllMagic`)
      (return true (`local.isMagic`))
      (else
        (switch `int` (`local.MagicType_0`)
          (:`1`
            ;[1 0 0.1108] FIRE
            (return (or (`self.FireAllLevels`) (and (`self.FireLevel_3`) (== (`local.MagicLvl_0`) 3)) (and (`self.FireLevel_2`) (or (== (`local.MagicLvl_0`) 3) (== (`local.MagicLvl_0`) 2))) (and (`self.FireLevel_1`) (or (== (`local.MagicLvl_0`) 3) (== (`local.MagicLvl_0`) 2) (== (`local.MagicLvl_0`) 1)))) (`local.isMagic`)))
          (:`2`
            ;[0 0.8263 1] ICE
            (return (or (`self.IceAllLevels`) (and (`self.IceLevel_3`) (== (`local.MagicLvl_0`) 3)) (and (`self.IceLevel_2`) (or (== (`local.MagicLvl_0`) 3) (== (`local.MagicLvl_0`) 2))) (and (`self.IceLevel_1`) (or (== (`local.MagicLvl_0`) 3) (== (`local.MagicLvl_0`) 2) (== (`local.MagicLvl_0`) 1)))) (`local.isMagic`)))
          (:`3`
            ;[0.9947 1 0.05294] LIGHTNING
            (return (or (`self.LightningAllLevels`) (and (`self.LightningLevel_3`) (== (`local.MagicLvl_0`) 3)) (and (`self.LightningLevel_2`) (or (== (`local.MagicLvl_0`) 3) (== (`local.MagicLvl_0`) 2))) (and (`self.LightningLevel_1`) (or (== (`local.MagicLvl_0`) 3) (== (`local.MagicLvl_0`) 2) (== (`local.MagicLvl_0`) 1)))) (`local.isMagic`))))))
    (else
      (return false false))))