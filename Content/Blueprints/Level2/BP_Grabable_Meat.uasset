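; BP_Grabable_Meat is a Level 2 meat object, apparently grabbable, that stays unavailable until a specific event reveals it.
; On BeginPlay it hides itself and turns off overlap events on its GrabZone.
; When its Event handler receives ID 4, it unhides the actor and re-enables GrabZone overlaps.
; The graph holds no grab logic of its own, and construction defers to the parent class.
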(event `self.ReceiveBeginPlay`
  (`self.SetActorHiddenInGame` true)
  (set `PrimitiveComponent.bGenerateOverlapEvents` false (`self.grabZone`)))

(event `/Game/Blueprints/Interfaces/BPI_EventReceiver.ReceiveEvent`
  (params (ID :type Integer))
  (if (== ID 4)
    (`self.SetActorHiddenInGame` false)
    (set `PrimitiveComponent.bGenerateOverlapEvents` true (`self.grabZone`))))

(fn `UserConstructionScript`
  (`parent.UserConstructionScript`))