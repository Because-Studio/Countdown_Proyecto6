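; BP_Interactuablelvl2 is a Level 2 interactable that stays locked until it receives message ID 3.
; Once unlocked, its object action spawns a scaled-up fire particle effect above the actor.
; After a delay it sends message ID 4, then destroys the fire shortly afterward.
; The unlock flag is never cleared here, so the action remains available afterward.
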(event `/Game/Blueprints/Interfaces/BPI_EventReceiver.ReceiveEvent`
  (params (ID :type Integer))
  (if (== ID 3)
    (set `self.canInteract?` true)))

(event `self.ObjectAction`
  (if (`self.canInteract?`)
    (bind _returnvalue (`GameplayStatics.SpawnEmitterAtLocation` "/Game/StarterContent/Particles/P_Fire.P_Fire" (+ (`self.K2_GetActorLocation`) (0.0 0.0 180.0)) (struct) (3.0 3.0 5.0)))
    (`KismetSystemLibrary.Delay` 5.0)
    (`/Game/Blueprints/Function/BPF_MessageWithID.SendMessageWithID` 4)
    (`KismetSystemLibrary.Delay` 2.0)
    (`ActorComponent.K2_DestroyComponent` _returnvalue)))

(fn `UserConstructionScript`
  (`parent.UserConstructionScript`))