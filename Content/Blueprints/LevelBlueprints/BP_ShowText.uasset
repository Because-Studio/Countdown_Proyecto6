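; BP_ShowText is a level actor that shows a piece of world-space text while the player stands inside its trigger area.
; On BeginPlay it caches the BP_Player character and writes its Text variable into a TextRender component.
; Box overlap events compare against that cached player, making the text visible on enter and hiding it on exit.
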(event `self.ReceiveBeginPlay`
  (bind _asbp_player (cast `/Game/Player/BP_Player` (`GameplayStatics.GetPlayerCharacter` 0)))
  (set `self.player` _asbp_player)
  (`TextRenderComponent.K2_SetText` (`self.TextRender`) (`self.Text`)))

(event `self.Box.OnComponentBeginOverlap`
  (params (OverlappedComponent :type "PrimitiveComponent Object Reference") (OtherActor :type "Actor Object Reference") (OtherComp :type "PrimitiveComponent Object Reference") (OtherBodyIndex :type Integer) (bFromSweep :type Boolean) (SweepResult :type "HitResult Structure (by ref)"))
  (if (== OtherActor (`self.player`))
    (`SceneComponent.SetVisibility` (`self.TextRender`) true false)))

(event `self.Box.OnComponentEndOverlap`
  (params (OverlappedComponent :type "PrimitiveComponent Object Reference") (OtherActor :type "Actor Object Reference") (OtherComp :type "PrimitiveComponent Object Reference") (OtherBodyIndex :type Integer))
  (if (== OtherActor (`self.player`))
    (`SceneComponent.SetVisibility` (`self.TextRender`) false false)))

(fn `UserConstructionScript`)