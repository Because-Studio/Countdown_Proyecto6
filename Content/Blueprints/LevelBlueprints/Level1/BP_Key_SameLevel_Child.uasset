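; BP_Key_SameLevel_Child is a Level 1 key actor that responds to magic overlaps by lighting up two grabbable objects.
; On BeginPlay it caches the BP_Grabable_Child and BP_Grabable_Child2 instances found by class.
; An overlap passing the magic interactable check, while the first grabbable's two-objects-changed-material flag is set, applies a pulsing hex material to both GrabZones.
; It then marks the light active and sends an ID message intended for the first grabbable.
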(event `self.ReceiveBeginPlay`
  (bind _returnvalue (`GameplayStatics.GetActorOfClass` "/Game/Blueprints/LevelBlueprints/Level1/BP_Grabable_Child.BP_Grabable_Child_C"))
  (set `self.BP_Grabable_Child` _returnvalue)
  (bind _returnvalue_2 (`GameplayStatics.GetActorOfClass` "/Game/Blueprints/LevelBlueprints/Level1/BP_Grabable_Child2.BP_Grabable_Child2_C"))
  (set `self.BP_Grabable_Child2` _returnvalue_2))

(event `self.ReceiveActorBeginOverlap`
  (params (OtherActor :type "Actor Object Reference"))
  (bind _condition_ (`/Game/Blueprints/BPComponents/BPC_MagicInteractuable.checkMagic` (`self.BPC_MagicInteractuable`) OtherActor))
  (if (and _condition_ (`/Game/Blueprints/LevelBlueprints/Level1/BP_Grabable_Child.2Objects_ChangedMaterial?` (`self.BP_Grabable_Child`)))
    (`PrimitiveComponent.SetMaterial` (`/Game/Blueprints/BP_Grabable.grabZone` (`self.BP_Grabable_Child`)) 0 "/Game/StarterContent/Materials/M_Tech_Hex_Tile_Pulse.M_Tech_Hex_Tile_Pulse")
    (`PrimitiveComponent.SetMaterial` (`/Game/Blueprints/BP_Grabable.grabZone` (`self.BP_Grabable_Child2`)) 0 "/Game/StarterContent/Materials/M_Tech_Hex_Tile_Pulse.M_Tech_Hex_Tile_Pulse")
    (set `self.lightActived?` true)
    ;[1 1 1] Int_0_To_grabableChild1
    (`/Game/Blueprints/Function/BPF_MessageWithID.SendMessageWithID` (`self.ID_0`))))

(fn `UserConstructionScript`
  (`parent.UserConstructionScript`))