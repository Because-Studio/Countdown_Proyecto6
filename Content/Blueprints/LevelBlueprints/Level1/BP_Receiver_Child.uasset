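; Level 1 key pickup, a child receiver actor that flags the level's door once collected.
; A message with a matching ID teleports it to a BP_Empty_MarkLocation actor found at BeginPlay.
; An overlap that passes the magic component's check turns its cube gold and makes it pickable.
; Its box enables input while the player overlaps, so Interact can destroy it and set KeyDestroyed on BP_Door.
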(event `self.ReceiveTick`
  (params (DeltaSeconds :type "Float (single-precision)")))

(event `self.ReceiveBeginPlay`
  (bind _returnvalue (`GameplayStatics.GetActorOfClass` "/Game/Blueprints/LevelBlueprints/Level1/BP_Empty_MarkLocation.BP_Empty_MarkLocation_C"))
  (set `self.Actor_MarkLocation` _returnvalue)
  (bind _asbp_player (cast `/Game/Player/BP_Player` (`GameplayStatics.GetPlayerCharacter` 0)))
  (set `self.BP Player` _asbp_player)
  (bind _returnvalue_2 (`GameplayStatics.GetActorOfClass` "/Game/Blueprints/BP_Door.BP_Door_C"))
  (set `self.BP_door` _returnvalue_2))

(event `/Game/Blueprints/Interfaces/BPI_EventReceiver.ReceiveEvent`
  (params (ID :type Integer))
  (bind _match_ (`/Game/Blueprints/Function/BPF_MessageWithID.ReceiveMessageWithID` ID (`self.ReceveID`)))
  (if _match_
    (`self.CE_SetLoc`)))

(event `CE_SetLoc`
  (`SceneComponent.K2_SetWorldLocation` (`self.DefaultSceneRoot`) (`self.K2_GetActorLocation` (`self.Actor_MarkLocation`)) false true))

(event `self.Box.OnComponentBeginOverlap`
  (params (OverlappedComponent :type "PrimitiveComponent Object Reference") (OtherActor :type "Actor Object Reference") (OtherComp :type "PrimitiveComponent Object Reference") (OtherBodyIndex :type Integer) (bFromSweep :type Boolean) (SweepResult :type "HitResult Structure (by ref)"))
  (if (== OtherActor (`self.BP Player`))
    (`self.EnableInput` (`GameplayStatics.GetPlayerController` 0))))

(event `InputAction|Interact`
  (params (Key :type "Key Structure"))
  (:`Pressed`
    (if (`self.keyCanPick?`)
      (`self.K2_DestroyActor`)
      (set `/Game/Blueprints/BP_Door.keyDestroyed?` true (`self.BP_door`)))))

(event `self.Box.OnComponentEndOverlap`
  (params (OverlappedComponent :type "PrimitiveComponent Object Reference") (OtherActor :type "Actor Object Reference") (OtherComp :type "PrimitiveComponent Object Reference") (OtherBodyIndex :type Integer))
  (if (== OtherActor (`self.BP Player`))
    (`self.DisableInput` (`GameplayStatics.GetPlayerController` 0))))

(event `self.ReceiveActorBeginOverlap`
  (params (OtherActor :type "Actor Object Reference"))
  (bind _condition_ (`/Game/Blueprints/BPComponents/BPC_MagicInteractuable.checkMagic` (`self.BPC_MagicInteractuable`) OtherActor))
  (if _condition_
    (`PrimitiveComponent.SetMaterial` (`self.Cube`) 0 "/Game/Fantastic_Village_Pack/materials/MI_gold.MI_gold")
    (set `self.keyCanPick?` true)))

(fn `UserConstructionScript`
  (`parent.UserConstructionScript`))