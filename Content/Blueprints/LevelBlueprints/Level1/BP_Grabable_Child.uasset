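; Level 1 grabbable child Blueprint forming one half of a two-object magic check with BP_Grabable_Child2, which it finds on BeginPlay.
; When a magic overlap passes BPCMagicInteractuable's check while either object-in-location flag is set, it turns GrabZone red and increments its index.
; It then sets a both-objects-changed flag if both its own and the partner's index have reached at least one.
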(event `self.ReceiveBeginPlay`
  (bind _returnvalue (`GameplayStatics.GetActorOfClass` "/Game/Blueprints/LevelBlueprints/Level1/BP_Grabable_Child2.BP_Grabable_Child2_C"))
  (set `self.Grabable2` _returnvalue))

(event `self.ReceiveActorBeginOverlap`
  (params (OtherActor :type "Actor Object Reference"))
  (`|ExecutionSequence`
    (:`then_0`
      (bind _condition_ (`/Game/Blueprints/BPComponents/BPC_MagicInteractuable.checkMagic` (`self.BPC_MagicInteractuable`) OtherActor))
      (if (and _condition_ (or (`self.object1_InLocation?`) (`self.object2_InLocarion?`)))
        (`PrimitiveComponent.SetMaterial` (`self.grabZone`) 0 "/Game/Material/M_Red.M_Red")
        (`/Engine/EditorBlueprintResources/StandardMacros.IncrementInt` (`self.Index_Control`)
          (:`  `
            (`self.CE_CheckIndex`)))))))

(event `CE_CheckIndex`
  (if (and (>= (`/Game/Blueprints/LevelBlueprints/Level1/BP_Grabable_Child2.Index_Control` (`self.Grabable2`)) 1) (>= (`self.Index_Control`) 1))
    (set `self.2Objects_ChangedMaterial?` true)))

(fn `UserConstructionScript`
  (`parent.UserConstructionScript`))