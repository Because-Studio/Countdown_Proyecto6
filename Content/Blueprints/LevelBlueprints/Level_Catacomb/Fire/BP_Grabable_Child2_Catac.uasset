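; BP_Grabable_Child2_Catac is a grabbable child Blueprint for a fire puzzle in the Catacomb level that opens a door.
; On BeginPlay it caches the fire effect, gear (Engranaje) and DoorFire2 actors by class.
; A magic overlap while the object is in location turns GrabZone red and increments a counter.
; The counter check spawns fire at the effect actor, then after a delay rotates the gear and opens the door.
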(event `self.ReceiveBeginPlay`
  (bind _returnvalue (`GameplayStatics.GetActorOfClass` "/Game/Blueprints/LevelBlueprints/Level_Catacomb/Fire/BP_FireEfect.BP_FireEfect_C"))
  (set `self.fireLocation` _returnvalue)
  (bind _returnvalue_2 (`GameplayStatics.GetActorOfClass` "/Game/Blueprints/LevelBlueprints/Level_Catacomb/Fire/BP_Engranaje.BP_Engranaje_C"))
  (set `self.engranaje` _returnvalue_2)
  (bind _returnvalue_3 (`GameplayStatics.GetActorOfClass` "/Game/Blueprints/LevelBlueprints/Level_Catacomb/Fire/BP_DoorFire2.BP_DoorFire2_C"))
  (set `self.doorFire2` _returnvalue_3))

(event `self.ReceiveActorBeginOverlap`
  (params (OtherActor :type "Actor Object Reference"))
  (`|ExecutionSequence`
    (:`then_0`
      (bind _condition_ (`/Game/Blueprints/BPComponents/BPC_MagicInteractuable.checkMagic` (`self.BPC_MagicInteractuable`) OtherActor))
      (if (and _condition_ (`self.object2_InLocarion?`))
        (`PrimitiveComponent.SetMaterial` (`self.grabZone`) 0 "/Game/Material/M_Red.M_Red")
        (`/Engine/EditorBlueprintResources/StandardMacros.IncrementInt` (`self.Index_Control`)
          (:`  `
            (`self.CE_CheckIndex`)))))))

(event `CE_CheckIndex`
  (if (>= (`self.Index_Control`) 1)
    (set `self.2Objects_ChangedMaterial?` true)
    (`GameplayStatics.SpawnEmitterAtLocation` "/Game/StarterContent/Particles/P_Fire.P_Fire" (`SceneComponent.K2_GetComponentLocation` (`/Game/Blueprints/LevelBlueprints/Level_Catacomb/Fire/BP_FireEfect.DefaultSceneRoot` (`self.fireLocation`))))
    (`KismetSystemLibrary.Delay` 1.5)
    (`/Game/Blueprints/LevelBlueprints/Level_Catacomb/Fire/BP_Engranaje.CE_RotaEnganaje` (`self.engranaje`))
    (`/Game/Blueprints/LevelBlueprints/Level_Catacomb/Fire/BP_DoorFire2.CE_OpenDoor` (`self.doorFire2`))))

(fn `UserConstructionScript`
  (`parent.UserConstructionScript`))