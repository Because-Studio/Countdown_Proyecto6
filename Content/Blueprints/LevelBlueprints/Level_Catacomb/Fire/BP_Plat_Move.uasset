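; Moving platform for the Catacomb fire level that slides its mesh back and forth along its relative Y axis until magic stops it.
; Two timelines, SetLoc and Re (played in reverse), drive the motion and restart each other on finish for an endless loop.
; An overlap that passes the BPCMagicInteractuable magic check turns the mesh red, disables the Box collision and stops both timelines, with no logic to resume.
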(event `self.ReceiveBeginPlay`
  (bind _staticmesh (`self.StaticMesh`))
  (bind (_direction _float) (`Timeline|SetLoc` :!label _label)
    (:`Update`
      (`SceneComponent.K2_SetRelativeLocation` _staticmesh (`KismetMathLibrary.MakeVector` 0.0 _float) false false))
    (:`Finished`
      (bind (_direction_2 _float_2) (`Timeline|Re` :!via `ReverseFromEnd` :!label _label_2)
        (:`Update`
          (`SceneComponent.K2_SetRelativeLocation` _staticmesh (`KismetMathLibrary.MakeVector` 0.0 _float_2) false false))
        (:`Finished`
          (goto _label :!via `PlayFromStart`))))))

(event `self.ReceiveActorBeginOverlap`
  (params (OtherActor :type "Actor Object Reference"))
  (bind _condition_ (`/Game/Blueprints/BPComponents/BPC_MagicInteractuable.checkMagic` (`self.BPC_MagicInteractuable`) OtherActor))
  (if _condition_
    (`PrimitiveComponent.SetMaterial` (`self.StaticMesh`) 0 "/Game/Material/M_Red.M_Red")
    (`PrimitiveComponent.SetCollisionEnabled` (`self.Box`) "NoCollision")
    (`|ExecutionSequence`
      (:`then_0`
        (goto _label :!via `Stop`))
      (:`then_1`
        (goto _label_2 :!via `Stop`)))))

(fn `UserConstructionScript`)