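; Child Blueprint of a grabbable object for the Catacomb level's fire section, with the beginnings of a two-object placement check.
; On BeginPlay it caches the BP_Grabable_Child3_Catac instance, and on overlap it runs the magic-interactable component's CheckMagic without using the result.
; CE_CheckIndex sets a both-objects flag once both IndexControl counters reach one.
; The red-material swap, counter increment and CECheckIndex call are disconnected.
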(event `self.ReceiveBeginPlay`
  (bind _returnvalue (`GameplayStatics.GetActorOfClass` "/Game/Blueprints/LevelBlueprints/Level_Catacomb/Fire/BP_Grabable_Child3_Catac.BP_Grabable_Child3_Catac_C"))
  (set `self.Grab2` _returnvalue))

(event `self.ReceiveActorBeginOverlap`
  (params (OtherActor :type "Actor Object Reference"))
  (`|ExecutionSequence`
    (:`then_0`
      (bind _condition_ (`/Game/Blueprints/BPComponents/BPC_MagicInteractuable.checkMagic` (`self.BPC_MagicInteractuable`) OtherActor)))))

(event `CE_CheckIndex`
  (if (and (>= (`/Game/Blueprints/LevelBlueprints/Level_Catacomb/Fire/BP_Grabable_Child3_Catac.Index_Control` (`self.Grab2`)) 1) (>= (`self.Index_Control`) 1))
    (set `self.2Objects_ChangedMaterial?` true)))

(fn `UserConstructionScript`
  (`parent.UserConstructionScript`))