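; BP_DoorFire1 is a door in the fire section of the Catacomb level that opens when its CE_OpenDoor custom event is called.
; The event plays the Down timeline, whose float track sets the relative Z of eight static mesh components each update, keeping their X and Y.
; All pieces share the same Z value; the file has no closing logic.
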(event `self.ReceiveBeginPlay`)

(event `CE_OpenDoor`
  (bind _staticmesh2 (`self.StaticMesh2`))
  (bind _staticmesh1 (`self.StaticMesh1`))
  (bind _staticmesh (`self.StaticMesh`))
  (bind _staticmesh4 (`self.StaticMesh4`))
  (bind _staticmesh5 (`self.StaticMesh5`))
  (bind _staticmesh6 (`self.StaticMesh6`))
  (bind _staticmesh7 (`self.StaticMesh7`))
  (bind _staticmesh3 (`self.StaticMesh3`))
  (bind (_relativelocation_x _relativelocation_y) (`KismetMathLibrary.BreakVector` (`SceneComponent.RelativeLocation` _staticmesh3)))
  (bind (_relativelocation_x_2 _relativelocation_y_2) (`KismetMathLibrary.BreakVector` (`SceneComponent.RelativeLocation` _staticmesh2)))
  (bind (_relativelocation_x_3 _relativelocation_y_3) (`KismetMathLibrary.BreakVector` (`SceneComponent.RelativeLocation` _staticmesh1)))
  (bind (_relativelocation_x_4 _relativelocation_y_4) (`KismetMathLibrary.BreakVector` (`SceneComponent.RelativeLocation` _staticmesh)))
  (bind (_relativelocation_x_5 _relativelocation_y_5) (`KismetMathLibrary.BreakVector` (`SceneComponent.RelativeLocation` _staticmesh4)))
  (bind (_relativelocation_x_6 _relativelocation_y_6) (`KismetMathLibrary.BreakVector` (`SceneComponent.RelativeLocation` _staticmesh5)))
  (bind (_relativelocation_x_7 _relativelocation_y_7) (`KismetMathLibrary.BreakVector` (`SceneComponent.RelativeLocation` _staticmesh6)))
  (bind (_relativelocation_x_8 _relativelocation_y_8) (`KismetMathLibrary.BreakVector` (`SceneComponent.RelativeLocation` _staticmesh7)))
  (bind (_direction _float) (`Timeline|Down`)
    (:`Update`
      (`SceneComponent.K2_SetRelativeLocation` _staticmesh2 (`KismetMathLibrary.MakeVector` _relativelocation_x_2 _relativelocation_y_2 _float) false false)
      (`SceneComponent.K2_SetRelativeLocation` _staticmesh1 (`KismetMathLibrary.MakeVector` _relativelocation_x_3 _relativelocation_y_3 _float) false false)
      (`SceneComponent.K2_SetRelativeLocation` _staticmesh (`KismetMathLibrary.MakeVector` _relativelocation_x_4 _relativelocation_y_4 _float) false false)
      (`SceneComponent.K2_SetRelativeLocation` _staticmesh4 (`KismetMathLibrary.MakeVector` _relativelocation_x_5 _relativelocation_y_5 _float) false false)
      (`SceneComponent.K2_SetRelativeLocation` _staticmesh5 (`KismetMathLibrary.MakeVector` _relativelocation_x_6 _relativelocation_y_6 _float) false false)
      (`SceneComponent.K2_SetRelativeLocation` _staticmesh6 (`KismetMathLibrary.MakeVector` _relativelocation_x_7 _relativelocation_y_7 _float) false false)
      (`SceneComponent.K2_SetRelativeLocation` _staticmesh7 (`KismetMathLibrary.MakeVector` _relativelocation_x_8 _relativelocation_y_8 _float) false false)
      (`SceneComponent.K2_SetRelativeLocation` _staticmesh3 (`KismetMathLibrary.MakeVector` _relativelocation_x _relativelocation_y _float) false false))))

(fn `UserConstructionScript`)