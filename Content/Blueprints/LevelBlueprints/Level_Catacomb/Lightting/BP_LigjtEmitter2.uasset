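; BP_LigjtEmitter2 is a Catacomb level coil emitter that activates a magnetic wall when touched by magic.
; On BeginPlay it caches the BP_Wall actor returned by GetActorOfClass.
; On overlap, if the BPCMagicInteractuable CheckMagic test passes, it switches its coil (Bobina) to a pulsing material, turns the wall yellow and enables the wall box's query and physics collision.
; Nothing in this Blueprint reverses the activation.
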(event `self.ReceiveBeginPlay`
  (bind _returnvalue (`GameplayStatics.GetActorOfClass` "/Game/Blueprints/LevelBlueprints/Level_Catacomb/Lightting/BP_Wall.BP_Wall_C"))
  (set `self.BP_Wall_Lightting` _returnvalue))

(event `self.ReceiveActorBeginOverlap`
  (params (OtherActor :type "Actor Object Reference"))
  (bind _condition_ (`/Game/Blueprints/BPComponents/BPC_MagicInteractuable.checkMagic` (`self.BPC_MagicInteractuable`) OtherActor))
  (if _condition_
    (`PrimitiveComponent.SetMaterial` (`self.bobina`) 0 "/Game/StarterContent/Materials/M_Tech_Hex_Tile_Pulse.M_Tech_Hex_Tile_Pulse")
    (`PrimitiveComponent.SetMaterial` (`/Game/Blueprints/LevelBlueprints/Level_Catacomb/Lightting/BP_Wall.ParedMagnetica` (`self.BP_Wall_Lightting`)) 0 "/Game/Material/M_Yellow.M_Yellow")
    (`PrimitiveComponent.SetCollisionEnabled` (`/Game/Blueprints/LevelBlueprints/Level_Catacomb/Lightting/BP_Wall.Box` (`self.BP_Wall_Lightting`)) "QueryAndPhysics")))

(fn `UserConstructionScript`)