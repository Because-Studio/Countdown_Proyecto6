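; BP_Wall is a Catacomb level actor with a Box trigger that turns off gravity and jumping for the player while inside it.
; BeginPlay caches the BP_Player reference and disables the Box's collision, which this Blueprint never re-enables.
; Overlap events zero the player's CharacterMovement gravity scale and jump velocity on entry, then set fixed values on exit rather than restoring saved ones.
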(event `self.ReceiveBeginPlay`
  (bind _asbp_player (cast `/Game/Player/BP_Player` (`GameplayStatics.GetPlayerCharacter` 0)))
  (set `self.BP Player` _asbp_player)
  (`PrimitiveComponent.SetCollisionEnabled` (`self.Box`) "NoCollision"))

(event `self.Box.OnComponentBeginOverlap`
  (params (OverlappedComponent :type "PrimitiveComponent Object Reference") (OtherActor :type "Actor Object Reference") (OtherComp :type "PrimitiveComponent Object Reference") (OtherBodyIndex :type Integer) (bFromSweep :type Boolean) (SweepResult :type "HitResult Structure (by ref)"))
  (bind _bp_player (`self.BP Player`))
  (bind _charactermovement (`Character.CharacterMovement` _bp_player))
  (if (== OtherActor _bp_player)
    (set `CharacterMovementComponent.GravityScale` 0.0 _charactermovement)
    (set `CharacterMovementComponent.JumpZVelocity` 0.0 _charactermovement)))

(event `self.Box.OnComponentEndOverlap`
  (params (OverlappedComponent :type "PrimitiveComponent Object Reference") (OtherActor :type "Actor Object Reference") (OtherComp :type "PrimitiveComponent Object Reference") (OtherBodyIndex :type Integer))
  (bind _bp_player (`self.BP Player`))
  (bind _charactermovement (`Character.CharacterMovement` _bp_player))
  (if (== OtherActor _bp_player)
    (set `CharacterMovementComponent.GravityScale` 1.5 _charactermovement)
    (set `CharacterMovementComponent.JumpZVelocity` 500.0 _charactermovement)))

(fn `UserConstructionScript`)