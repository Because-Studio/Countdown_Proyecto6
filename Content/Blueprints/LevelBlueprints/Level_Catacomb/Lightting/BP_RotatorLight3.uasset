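; BP_RotatorLight3 is a rotating mesh in the Catacomb level that responds to magic and depends on a BP_RotatorLight2 actor found on BeginPlay.
; A timeline pitches the mesh from the start of play.
; A magic overlap, valid only once Rote2Done is set on that light, resets the rotation and stops that timeline.
; After a brief delay, a one-shot second timeline drives the pitch and turns the material yellow.
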(event `self.ReceiveBeginPlay`
  (bind _returnvalue (`GameplayStatics.GetActorOfClass` "/Game/Blueprints/LevelBlueprints/Level_Catacomb/Lightting/BP_RotatorLight2.BP_RotatorLight2_C"))
  (set `self.rota2` _returnvalue)
  (bind (_direction _float) (`Timeline|Rote` :!via `PlayFromStart` :!label _label)
    (:`Update`
      (`SceneComponent.K2_SetRelativeRotation` (`self.StaticMesh`) (`KismetMathLibrary.MakeRotator` 0.0 _float) false false))))

(event `self.ReceiveActorBeginOverlap`
  (params (OtherActor :type "Actor Object Reference"))
  (bind _staticmesh (`self.StaticMesh`))
  (bind (_relativerotation_roll _relativerotation_pitch _relativerotation_yaw) (`KismetMathLibrary.BreakRotator` (`SceneComponent.RelativeRotation` _staticmesh)))
  (bind _condition_ (`/Game/Blueprints/BPComponents/BPC_MagicInteractuable.checkMagic` (`self.BPC_MagicInteractuable`) OtherActor))
  (if _condition_
    (if (`/Game/Blueprints/LevelBlueprints/Level_Catacomb/Lightting/BP_RotatorLight2.rote2Done?` (`self.rota2`))
      (`|ExecutionSequence`
        (:`then_0`
          (`SceneComponent.K2_SetRelativeRotation` :`self` (`self.StaticMesh`))
          (goto _label :!via `Stop`))
        (:`then_1`
          (`KismetSystemLibrary.Delay` 0.1)
          (`/Engine/EditorBlueprintResources/StandardMacros.DoOnce` false
            (:`Completed`
              (bind (_direction _newtrack_0) (`Timeline|Ro` :!via `PlayFromStart`)
                (:`Update`
                  (`SceneComponent.K2_SetRelativeRotation` _staticmesh (`KismetMathLibrary.MakeRotator` _relativerotation_roll _newtrack_0 _relativerotation_yaw) false false)
                  (`PrimitiveComponent.SetMaterial` _staticmesh 0 "/Game/Material/M_Yellow.M_Yellow"))))))))))

(fn `UserConstructionScript`)