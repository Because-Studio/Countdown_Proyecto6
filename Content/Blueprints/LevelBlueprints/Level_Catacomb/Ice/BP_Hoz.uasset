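; BP_Hoz is a swinging scythe hazard in the Catacomb ice level that teleports the player to the BP_EmpActor_Hielo location on overlap.
; The Rota timeline drives the blade's pitch from BeginPlay.
; When an overlap on its Box passes the BPCMagicInteractuable magic check, Rota stops and a second timeline takes over the pitch, disabling Box collision and swapping the blade to a blue debug material.
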(event `self.ReceiveBeginPlay`
  (bind _asbp_player (cast `/Game/Player/BP_Player` (`GameplayStatics.GetPlayerCharacter` 0)))
  (set `self.BP Player` _asbp_player)
  (bind _returnvalue (`GameplayStatics.GetActorOfClass` "/Game/Blueprints/LevelBlueprints/Level_Catacomb/BP_EmpActor_Hielo.BP_EmpActor_Hielo_C"))
  (set `self.ActorHielo` _returnvalue)
  (bind (_direction _newtrack_0) (`Timeline|rota` :!label _label)
    (:`Update`
      (`SceneComponent.K2_SetRelativeRotation` (`self.Hoz`) (`KismetMathLibrary.MakeRotator` 0.0 _newtrack_0) false false))))

(event `self.Box.OnComponentBeginOverlap`
  (params (OverlappedComponent :type "PrimitiveComponent Object Reference") (OtherActor :type "Actor Object Reference") (OtherComp :type "PrimitiveComponent Object Reference") (OtherBodyIndex :type Integer) (bFromSweep :type Boolean) (SweepResult :type "HitResult Structure (by ref)"))
  (bind _condition_ (`/Game/Blueprints/BPComponents/BPC_MagicInteractuable.checkMagic` (`self.BPC_MagicInteractuable`) OtherActor))
  (if _condition_
    (`|ExecutionSequence`
      (:`then_0`
        (goto _label :!via `Stop`))
      (:`then_1`
        (bind (_direction _newtrack_0) (`Timeline|Timeline_0`)
          (:`Update`
            (`SceneComponent.K2_SetRelativeRotation` (`self.Hoz`) (`KismetMathLibrary.MakeRotator` 0.0 _newtrack_0) false false)
            (`PrimitiveComponent.SetCollisionEnabled` (`self.Box`) "NoCollision")
            (`PrimitiveComponent.SetMaterial` (`self.Hoz`) 0 "/Game/Material/VertexColorViewMode_BlueOnly.VertexColorViewMode_BlueOnly")))))))

(event `self.ReceiveActorBeginOverlap`
  (params (OtherActor :type "Actor Object Reference"))
  (if (== OtherActor (`self.BP Player`))
    (`self.K2_SetActorLocation` (`self.BP Player`) (`self.K2_GetActorLocation` (`self.ActorHielo`)) false true)))

(fn `UserConstructionScript`)