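; Trigger volume in the Catacomb level that lets the player create ice cubes on water.
; While the player is inside, a looping timer traces from the spine socket along ActorForAngle's forward vector.
; Hitting BP_Water enables the trigger's input and shows the player's preview cube; other results disable input.
; Holding Interact briefly spawns an ice cube at the impact point, grown by the Scale timeline until release stops it.
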(event `self.ReceiveBeginPlay`
  (bind _asbp_player (cast `/Game/Player/BP_Player` (`GameplayStatics.GetPlayerCharacter` 0)))
  (set `self.BP Player` _asbp_player)
  (bind _returnvalue (`GameplayStatics.GetActorOfClass` "/Game/Blueprints/LevelBlueprints/Level_Catacomb/Ice/BP_Water.BP_Water_C"))
  (set `self.BP_Water` _returnvalue))

(event `self.Box.OnComponentBeginOverlap`
  (params (OverlappedComponent :type "PrimitiveComponent Object Reference") (OtherActor :type "Actor Object Reference") (OtherComp :type "PrimitiveComponent Object Reference") (OtherBodyIndex :type Integer) (bFromSweep :type Boolean) (SweepResult :type "HitResult Structure (by ref)"))
  (if (== OtherActor (`self.BP Player`))
    (bind _returnvalue (`KismetSystemLibrary.K2_SetTimerDelegate` (delegate `CE_Trace`) 0.1 true))))

(event `CE_Trace`
  (bind _bp_player (`self.BP Player`))
  (bind _cube (`/Game/Player/BP_Player.Cube` (`self.BP Player`)))
  (bind _returnvalue (`SceneComponent.GetSocketLocation` (`Character.Mesh` _bp_player) "socket_spine5"))
  (bind _outhit (`KismetSystemLibrary.LineTraceSingle` _returnvalue (+ (* (`SceneComponent.GetForwardVector` (`/Game/Player/BP_Player.actorForAngle` _bp_player)) (`KismetMathLibrary.Conv_DoubleToVector` 1000.0)) _returnvalue) "TraceTypeQuery1"))
  (if (== (`.HitActor` (`GameplayStatics.BreakHitResult` _outhit)) (`self.BP_Water`))
    (`self.EnableInput` (`GameplayStatics.GetPlayerController` 0))
    (`SceneComponent.K2_SetWorldLocation` _cube (`.Location` (`GameplayStatics.BreakHitResult` _outhit)) false false)
    (`SceneComponent.SetVisibility` _cube true false)
    (else
      (`self.DisableInput` (`GameplayStatics.GetPlayerController` 0)))))

(event `self.Box.OnComponentEndOverlap`
  (params (OverlappedComponent :type "PrimitiveComponent Object Reference") (OtherActor :type "Actor Object Reference") (OtherComp :type "PrimitiveComponent Object Reference") (OtherBodyIndex :type Integer))
  (if (== OtherActor (`self.BP Player`))
    (`KismetSystemLibrary.K2_ClearAndInvalidateTimerHandle` (stale `self.Box.OnComponentBeginOverlap` _returnvalue))
    (`SceneComponent.SetVisibility` (`/Game/Player/BP_Player.Cube` (`self.BP Player`)) false false)))

(event `InputAxis|GenerateHieloCube`
  (params (AxisValue :type "Float (single-precision)")))

(event `InputAction|Interact`
  (params (Key :type "Key Structure"))
  (:`Pressed`
    (`KismetSystemLibrary.PrintString` "Hello")
    (bind _returnvalue (`KismetSystemLibrary.K2_SetTimerDelegate` (delegate `CE_GeneraCube`) 0.1)))
  (:`Released`
    (`KismetSystemLibrary.PrintString` "1111111111o")
    (`KismetSystemLibrary.K2_ClearAndInvalidateTimerHandle` _returnvalue)
    (bind (_direction _newtrack_0) (`Timeline|scale` :!via `Stop` :!label _label)
      (:`Update`
        (`self.SetActorScale3D` (stale `CE_GeneraCube` _returnvalue) (`KismetMathLibrary.Conv_DoubleToVector` _newtrack_0))))))

(event `CE_GeneraCube`
  (bind _returnvalue (`|SpawnActorFromClass` "/Game/Blueprints/LevelBlueprints/Level_Catacomb/Ice/BP_IceCube.BP_IceCube_C" (`KismetMathLibrary.Conv_VectorToTransform` (`.ImpactPoint` (`GameplayStatics.BreakHitResult` (stale `CE_Trace` _outhit)))) "Undefined" "OverrideRootScale" null null))
  (goto _label :!via `PlayFromStart`))

(fn `UserConstructionScript`)