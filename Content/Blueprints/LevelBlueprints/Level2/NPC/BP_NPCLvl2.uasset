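; BP_NPCLvl2 is a talkable Level 2 NPC whose dialogue changes as the player progresses.
; An ID-driven Event swaps the BPCTalkableNPC component's dialogue tree, or destroys the NPC after a short delay.
; Overlapping a grabbable meat actor destroys the meat and switches the NPC to another dialogue tree.
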(event `/Game/Blueprints/Interfaces/BPI_EventReceiver.ReceiveEvent`
  (params (ID :type Integer))
  (if (== ID 0)
    (set `/Game/Blueprints/BPComponents/BPC_TalkableNPC.DialogueTree` "/Game/Blueprints/LevelBlueprints/Level2/NPC/Dialogue2_NPC1.Dialogue2_NPC1" (`self.BPC_TalkableNPC`))
    (elif (== ID 2)
      (set `/Game/Blueprints/BPComponents/BPC_TalkableNPC.DialogueTree` "/Game/Blueprints/LevelBlueprints/Level2/NPC/Dialogue3_NPC1.Dialogue3_NPC1" (`self.BPC_TalkableNPC`))
      (elif (== ID 5)
        (`KismetSystemLibrary.Delay` 0.1)
        (`self.K2_DestroyActor`)))))

(event `self.ReceiveActorBeginOverlap`
  (params (OtherActor :type "Actor Object Reference"))
  (if (== (`GameplayStatics.GetObjectClass` OtherActor) "/Game/Blueprints/LevelBlueprints/Level2/BP_Grabable_Meat.BP_Grabable_Meat_C")
    (`self.K2_DestroyActor` OtherActor)
    (set `/Game/Blueprints/BPComponents/BPC_TalkableNPC.DialogueTree` "/Game/Blueprints/LevelBlueprints/Level2/NPC/Dialogue4_NPC1.Dialogue4_NPC1" (`self.BPC_TalkableNPC`))))

(fn `UserConstructionScript`
  (`parent.UserConstructionScript`))