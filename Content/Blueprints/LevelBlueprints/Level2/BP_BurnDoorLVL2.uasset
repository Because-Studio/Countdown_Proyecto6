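; Level 2 door that burns away when its ObjectAction event is triggered.
; The event spawns an enlarged P_Fire emitter at the door's location, then hides the door after a short delay.
; After a second delay it destroys the actor, then calls DestroyComponent on the fire emitter.
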(event `self.ObjectAction`
  (bind _returnvalue (`GameplayStatics.SpawnEmitterAtLocation` "/Game/StarterContent/Particles/P_Fire.P_Fire" (`self.K2_GetActorLocation`) (struct) (5.0 5.0 5.0)))
  (`KismetSystemLibrary.Delay` 1.5)
  (`self.SetActorHiddenInGame` true)
  (`KismetSystemLibrary.Delay` 0.7)
  (`self.K2_DestroyActor`)
  (`ActorComponent.K2_DestroyComponent` _returnvalue))

(fn `UserConstructionScript`
  (`parent.UserConstructionScript`))