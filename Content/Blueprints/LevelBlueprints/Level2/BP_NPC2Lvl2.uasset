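; BP_NPC2Lvl2 is a talkable NPC for Level 2 whose dialogue and presence change with story events.
; Its Event graph branches on an ID to swap the DialogueTree on its BPCTalkableNPC component between an opening and an ending dialogue.
; A later ID destroys the actor, and the construction script only calls its parent.
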(event `/Game/Blueprints/Interfaces/BPI_EventReceiver.ReceiveEvent`
  (params (ID :type Integer))
  (if (== ID 0)
    (set `/Game/Blueprints/BPComponents/BPC_TalkableNPC.DialogueTree` "/Game/Blueprints/LevelBlueprints/Level2/Dialogue1_NPC2.Dialogue1_NPC2" (`self.BPC_TalkableNPC`))
    (elif (== ID 2)
      (set `/Game/Blueprints/BPComponents/BPC_TalkableNPC.DialogueTree` "/Game/Blueprints/LevelBlueprints/Level2/DialogueEnd_NPC2.DialogueEnd_NPC2" (`self.BPC_TalkableNPC`))
      (elif (== ID 5)
        (`self.K2_DestroyActor`)))))

(fn `UserConstructionScript`
  (`parent.UserConstructionScript`))