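; BP_Interactuablelvl2 is a Level 2 interactable that stays inactive until its ID event receives 3.
; Once enabled, its ObjectAction spawns a scaled fire effect above the actor, sends message ID 4 after a delay, then removes the effect.
; Overlapping BP_GeneralFoodLvl2 actors are destroyed and counted as Apples while it is enabled, but that count does not gate the action.
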(event `/Game/Blueprints/Interfaces/BPI_EventReceiver.ReceiveEvent`
  (params (ID :type Integer))
  (if (== ID 3)
    (set `self.canInteract?` true)))

(event `self.ObjectAction`
  (if (`self.canInteract?`)
    (bind _returnvalue (`GameplayStatics.SpawnEmitterAtLocation` "/Game/StarterContent/Particles/P_Fire.P_Fire" (+ (`self.K2_GetActorLocation`) (0.0 0.0 180.0)) (struct) (3.0 3.0 5.0)))
    (`KismetSystemLibrary.Delay` 5.0)
    (`/Game/Blueprints/Function/BPF_MessageWithID.SendMessageWithID` 4)
    (`KismetSystemLibrary.Delay` 2.0)
    (`ActorComponent.K2_DestroyComponent` _returnvalue)))

(event `self.ReceiveActorBeginOverlap`
  (params (OtherActor :type "Actor Object Reference"))
  (`parent.ReceiveActorBeginOverlap` OtherActor)
  (if (and (`self.canInteract?`) (== (`GameplayStatics.GetObjectClass` OtherActor) "/Game/Blueprints/LevelBlueprints/Level2/BP_GeneralFoodLvl2.BP_GeneralFoodLvl2_C"))
    (`/Engine/EditorBlueprintResources/StandardMacros.IncrementInt` (`self.apples`)
      (:`  `
        (`self.K2_DestroyActor` OtherActor)))))

(fn `UserConstructionScript`
  (`parent.UserConstructionScript`))