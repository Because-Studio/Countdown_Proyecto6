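; BP_Door_LVL2 is a Level 2 door that loads the Village level once it is unlocked.
; An incoming Event with ID 6 sets CanOpen, which gates the door.
; Pressing Interact prints a debug string, then either plays a sound and opens Village after a short delay, or plays a different sound while locked.
; The Interact handler has no overlap or proximity check.
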(event `/Game/Blueprints/Interfaces/BPI_EventReceiver.ReceiveEvent`
  (params (ID :type Integer))
  (if (== ID 6)
    (set `self.canOpen?` true)))

(event `InputAction|Interact`
  (params (Key :type "Key Structure"))
  (:`Pressed`
    (`KismetSystemLibrary.PrintString` "Hello")
    (if (`self.canOpen?`)
      (`GameplayStatics.PlaySound2D` "/Game/Sounds/Dockable_Window_Drop.Dockable_Window_Drop" 1.0 1.0 0.0 null null)
      (`KismetSystemLibrary.Delay` 0.2)
      (`GameplayStatics.OpenLevel` "Village")
      (else
        (`GameplayStatics.PlaySound2D` "/Game/Sounds/EndPlayInEditor.EndPlayInEditor" 1.0 1.0 0.0 null null)))))

(fn `UserConstructionScript`
  (`parent.UserConstructionScript`))