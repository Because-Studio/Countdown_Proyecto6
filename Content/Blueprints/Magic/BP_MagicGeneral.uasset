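; BP_MagicGeneral is a magic actor, apparently a general projectile or spell, that bursts on contact.
; When its Col component begins overlapping anything other than player 0's pawn, it spawns an emitter effect at the Niagara component's location and destroys itself.
; Without such a hit, it destroys itself seven seconds after BeginPlay.
; The graph applies no damage and contains no movement logic.
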(event `self.ReceiveBeginPlay`
  (`KismetSystemLibrary.Delay` 7.0)
  (`self.K2_DestroyActor`))

(event `self.Col.OnComponentBeginOverlap`
  (params (OverlappedComponent :type "PrimitiveComponent Object Reference") (OtherActor :type "Actor Object Reference") (OtherComp :type "PrimitiveComponent Object Reference") (OtherBodyIndex :type Integer) (bFromSweep :type Boolean) (SweepResult :type "HitResult Structure (by ref)"))
  (if (not (== (`GameplayStatics.GetPlayerPawn` 0) OtherActor))
    (`GameplayStatics.SpawnEmitterAtLocation` (`self.Emitter Template`) (`SceneComponent.K2_GetComponentLocation` (`self.Niagara`)))
    (`self.K2_DestroyActor`)))

(fn `UserConstructionScript`)