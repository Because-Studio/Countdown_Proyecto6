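; BP_MagicGeneralHOLDED is a magic actor that, judging by its name, serves as a general held spell dealing periodic hits.
; On BeginPlay it pulses actor collision on for one tick, then a looping timer repeats that pulse every TimeToHit.
; An unconnected fragment would spawn an emitter at the Niagara component and destroy the actor after a player-pawn check, but it never runs.
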(event `self.ReceiveBeginPlay`
  (`self.SetActorEnableCollision` true)
  (`KismetSystemLibrary.DelayUntilNextTick`)
  (`self.SetActorEnableCollision` false)
  (`KismetSystemLibrary.K2_SetTimerDelegate` (delegate `CustomEventTick`) (`self.TimeToHit`) true))

(event `CustomEventTick`
  (`self.SetActorEnableCollision` true)
  (`KismetSystemLibrary.DelayUntilNextTick`)
  (`self.SetActorEnableCollision` false))

(fn `UserConstructionScript`)