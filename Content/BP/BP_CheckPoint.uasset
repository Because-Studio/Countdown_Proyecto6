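; BP_CheckPoint is a checkpoint actor that saves progress state when the player character overlaps its static mesh.
; On BeginPlay it caches the player character and the game instance.
; On overlap it flags PlayerInCheck on the game instance and stores the checkpoint's location plus the mesh locations of the first BP_Key1, BP_Key2 and BP_Key3 actors, printing each key location.
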(event `self.ReceiveBeginPlay`
  (bind _asbp_top_down_character (cast `/Game/TopDown/Blueprints/BP_TopDownCharacter` (`GameplayStatics.GetPlayerCharacter` 0)))
  (set `self.Player` _asbp_top_down_character)
  (bind _asbp_game_instance (cast `/Game/Blueprints/GameInstance/BP_GameInstance` (`GameplayStatics.GetGameInstance`)))
  (set `self.Game Instance` _asbp_game_instance))

(event `self.StaticMesh.OnComponentBeginOverlap`
  (params (OverlappedComponent :type "PrimitiveComponent Object Reference") (OtherActor :type "Actor Object Reference") (OtherComp :type "PrimitiveComponent Object Reference") (OtherBodyIndex :type Integer) (bFromSweep :type Boolean) (SweepResult :type "HitResult Structure (by ref)"))
  (if (== OtherActor (`self.Player`))
    (set `/Game/Blueprints/GameInstance/BP_GameInstance.PlayerInCheck?` true (`self.Game Instance`))
    (`|ExecutionSequence`
      (:`then_0`
        (bind _outactors (`GameplayStatics.GetAllActorsOfClass` "/Game/BP/BP_Key1.BP_Key1_C"))
        (bind _output_get (set `/Game/Blueprints/GameInstance/BP_GameInstance.key1Loc` (`SceneComponent.K2_GetComponentLocation` (`/Game/BP/BP_Key1.StaticMesh` (`|GetArrayItem` _outactors))) (`self.Game Instance`)))
        (`KismetSystemLibrary.PrintString` (`KismetStringLibrary.Conv_VectorToString` _output_get)))
      (:`then_1`
        (bind _outactors_2 (`GameplayStatics.GetAllActorsOfClass` "/Game/BP/BP_Key2.BP_Key2_C"))
        (bind _output_get_2 (set `/Game/Blueprints/GameInstance/BP_GameInstance.key2Loc` (`SceneComponent.K2_GetComponentLocation` (`/Game/BP/BP_Key2.StaticMesh` (`|GetArrayItem` _outactors_2))) (`self.Game Instance`)))
        (`KismetSystemLibrary.PrintString` (`KismetStringLibrary.Conv_VectorToString` _output_get_2)))
      (:`then_2`
        (bind _outactors_3 (`GameplayStatics.GetAllActorsOfClass` "/Game/BP/BP_Key3.BP_Key3_C"))
        (bind _output_get_3 (set `/Game/Blueprints/GameInstance/BP_GameInstance.key3Loc` (`SceneComponent.K2_GetComponentLocation` (`/Game/BP/BP_Key3.StaticMesh` (`|GetArrayItem` _outactors_3))) (`self.Game Instance`)))
        (`KismetSystemLibrary.PrintString` (`KismetStringLibrary.Conv_VectorToString` _output_get_3)))
      (:`then_3`
        (set `/Game/Blueprints/GameInstance/BP_GameInstance.CheckLoc` (`SceneComponent.K2_GetComponentLocation` (`self.StaticMesh`)) (`self.Game Instance`))))))

(fn `UserConstructionScript`)