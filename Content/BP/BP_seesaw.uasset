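; BP_seesaw is a seesaw actor that tilts when a BP_IceCube enters one of its two trigger boxes.
; Each box's overlap compares the entering actor against all BP_IceCube instances, then disables physics simulation on the static mesh and plays that box's timeline.
; Each timeline's Rota track is added as a local pitch delta on every update, so rotation accumulates.
; Nothing in the graph re-enables physics afterward.
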(event `self.Box.OnComponentBeginOverlap`
  (params (OverlappedComponent :type "PrimitiveComponent Object Reference") (OtherActor :type "Actor Object Reference") (OtherComp :type "PrimitiveComponent Object Reference") (OtherBodyIndex :type Integer) (bFromSweep :type Boolean) (SweepResult :type "HitResult Structure (by ref)"))
  (bind _outactors (`GameplayStatics.GetAllActorsOfClass` "/Game/BP/BP_IceCube.BP_IceCube_C"))
  (for _array_element _outactors
    (if (== OtherActor _array_element)
      (`PrimitiveComponent.SetSimulatePhysics` (`self.StaticMesh`) false)
      (bind (_direction _rota) (`Timeline|Timeline_0`)
        (:`Update`
          (`SceneComponent.K2_AddLocalRotation` (`self.StaticMesh`) (`KismetMathLibrary.MakeRotator` 0.0 _rota) false false))))))

(event `self.Box1.OnComponentBeginOverlap`
  (params (OverlappedComponent :type "PrimitiveComponent Object Reference") (OtherActor :type "Actor Object Reference") (OtherComp :type "PrimitiveComponent Object Reference") (OtherBodyIndex :type Integer) (bFromSweep :type Boolean) (SweepResult :type "HitResult Structure (by ref)"))
  (bind _outactors (`GameplayStatics.GetAllActorsOfClass` "/Game/BP/BP_IceCube.BP_IceCube_C"))
  (for _array_element _outactors
    (if (== OtherActor _array_element)
      (`PrimitiveComponent.SetSimulatePhysics` (`self.StaticMesh`) false)
      (bind (_direction _rota) (`Timeline|Timeline_1`)
        (:`Update`
          (`SceneComponent.K2_AddLocalRotation` (`self.StaticMesh`) (`KismetMathLibrary.MakeRotator` 0.0 _rota) false false))))))

(fn `UserConstructionScript`)