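; BP_Ice_fantasma_Oculta is an NPC that shows a line-by-line dialogue.
; Its sphere enables input while the player character overlaps and disables the player controller's input on exit.
; Each Talk call increments TalkIndex, then loops over Sound, playing every entry and setting the WB_Dialogue text, creating the widget if needed.
; Once the index passes the last line, it removes the widget and sets EndTalk.
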(event `/Game/BP/BP_Dialog.Talk`
  (`KismetSystemLibrary.PrintString` "Hello")
  (`/Engine/EditorBlueprintResources/StandardMacros.IncrementInt` (`self.talkIndex`)
    (:`  `
      (if (< (`self.talkIndex`) (`KismetArrayLibrary.Array_Length` (`self.Dialogue`)))
        (for _array_element (`self.sound`)
          (`GameplayStatics.PlaySound2D` _array_element 1.0 1.0 0.0 null null)
          (`self.UI`
            (:`then`
              _)
            (:`else`
              (bind _returnvalue (`|CreateWidget` "/Game/BP/UI/WB_Dialogue.WB_Dialogue_C" (`GameplayStatics.GetPlayerController` 0)))
              (bind _output_get (set `self.UI` _returnvalue))
              (`UserWidget.AddToViewport` _output_get 0)))
          (`TextBlock.SetText` (`/Game/BP/UI/WB_Dialogue.TextBlock_0` (`self.UI`)) (`KismetTextLibrary.Conv_StringToText` (`|GetArrayItem` (`self.Dialogue`) (`self.talkIndex`)))))
        (else
          (`Widget.RemoveFromParent` (`self.UI`))
          (set `self.endTalk?` true))))))

(event `self.ReceiveBeginPlay`
  (bind _asbp_top_down_character (cast `/Game/TopDown/Blueprints/BP_TopDownCharacter` (`GameplayStatics.GetPlayerCharacter` 0)))
  (set `self.player` _asbp_top_down_character))

(event `self.Sphere.OnComponentBeginOverlap`
  (params (OverlappedComponent :type "PrimitiveComponent Object Reference") (OtherActor :type "Actor Object Reference") (OtherComp :type "PrimitiveComponent Object Reference") (OtherBodyIndex :type Integer) (bFromSweep :type Boolean) (SweepResult :type "HitResult Structure (by ref)"))
  (if (== OtherActor (`self.player`))
    (`self.EnableInput` (`GameplayStatics.GetPlayerController` 0))
    (`KismetSystemLibrary.PrintString` "DoorIn")))

(event `self.Sphere.OnComponentEndOverlap`
  (params (OverlappedComponent :type "PrimitiveComponent Object Reference") (OtherActor :type "Actor Object Reference") (OtherComp :type "PrimitiveComponent Object Reference") (OtherBodyIndex :type Integer))
  (if (== OtherActor (`self.player`))
    (`self.DisableInput` (`GameplayStatics.GetPlayerController` 0) null)
    (`KismetSystemLibrary.PrintString` "DoorOut")))

(fn `UserConstructionScript`)