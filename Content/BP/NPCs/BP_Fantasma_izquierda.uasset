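; Left-side ghost NPC ("Fantasma izquierda") that talks to the player when the game instance's power is on.
; Sphere overlap enables actor input, and leaving calls DisableInput on the player controller.
; Each Talk call advances the dialogue, playing the sound array and updating a widget, then removes it and sets FinishTalk.
; Material-swap logic tied to light and power is unwired, so the CE_Dispear timer never starts.
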(event `self.ReceiveBeginPlay`
  (bind _asbp_top_down_character (cast `/Game/TopDown/Blueprints/BP_TopDownCharacter` (`GameplayStatics.GetPlayerCharacter` 0)))
  (set `self.Player` _asbp_top_down_character)
  (bind _asbp_game_instance (cast `/Game/Blueprints/GameInstance/BP_GameInstance` (`GameplayStatics.GetGameInstance`)))
  (set `self.As BP Game Instance` _asbp_game_instance))

(event `/Game/BP/BP_Dialog.Talk`
  (if (`/Game/Blueprints/GameInstance/BP_GameInstance.IsPowerOn?` (`self.As BP Game Instance`))
    (`/Engine/EditorBlueprintResources/StandardMacros.IncrementInt` (`self.talkIndex`)
      (:`  `
        (if (< (`self.talkIndex`) (`KismetArrayLibrary.Array_Length` (`self.Dialogue`)))
          (for _array_element (`self.sound`)
            (`GameplayStatics.PlaySound2D` _array_element 1.0 1.0 0.0 null null)
            (`self.UI`
              (:`then`
                _)
              (:`else`
                (bind _returnvalue (`|CreateWidget` null (`GameplayStatics.GetPlayerController` 0)))
                (bind _output_get (set `self.UI` _returnvalue))
                (`UserWidget.AddToViewport` _output_get 0)))
            (`TextBlock.SetText` (`/Game/BP/NPCs/BP_Fantasma_izquierda.TextBlock_0` (`self.UI`)) (`KismetTextLibrary.Conv_StringToText` (`|GetArrayItem` (`self.Dialogue`) (`self.talkIndex`)))))
          (else
            (`Widget.RemoveFromParent` (`self.UI`))
            (set `self.finishTalk?` true)))))))

(event `self.Sphere.OnComponentBeginOverlap`
  (params (OverlappedComponent :type "PrimitiveComponent Object Reference") (OtherActor :type "Actor Object Reference") (OtherComp :type "PrimitiveComponent Object Reference") (OtherBodyIndex :type Integer) (bFromSweep :type Boolean) (SweepResult :type "HitResult Structure (by ref)"))
  (if (== OtherActor (`self.Player`))
    (`self.EnableInput` (`GameplayStatics.GetPlayerController` 0))))

(event `CE_Dispear`
  ;[1 1 1] Dispear
  (if (not (or (`/Game/TopDown/Blueprints/BP_TopDownCharacter.IsLightting?` (`self.Player`)) (`/Game/Blueprints/GameInstance/BP_GameInstance.IsPowerOn?` (`self.As BP Game Instance`))))
    (`PrimitiveComponent.SetMaterial` (`self.SkeletalMesh`) 0 "/Game/StarterContent/Particles/Materials/M_Radial_Gradient.M_Radial_Gradient")))

(event `self.Sphere.OnComponentEndOverlap`
  (params (OverlappedComponent :type "PrimitiveComponent Object Reference") (OtherActor :type "Actor Object Reference") (OtherComp :type "PrimitiveComponent Object Reference") (OtherBodyIndex :type Integer))
  ;[1 1 1] Dispear
  (if (== OtherActor (`self.Player`))
    (`self.DisableInput` (`GameplayStatics.GetPlayerController` 0) null)))

(fn `UserConstructionScript`)