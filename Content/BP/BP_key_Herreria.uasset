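; BP_key_Herreria is a key pickup, apparently for the smithy, that the player removes by pressing E within its sphere.
; Sphere begin overlap enables input only for the first BP_Hielo actor found, while end overlap disables it for the cached BP_TopDownCharacter player, both playing the same sound.
; Pressing E triggers a custom destroy event that plays a sound and destroys the actor, without recording the key anywhere.
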(event `self.ReceiveBeginPlay`
  (bind _asbp_top_down_character (cast `/Game/TopDown/Blueprints/BP_TopDownCharacter` (`GameplayStatics.GetPlayerCharacter` 0)))
  (set `self.Player` _asbp_top_down_character))

(event `InputAction|Input(E)`
  (params (Key :type "Key Structure"))
  (:`Pressed`
    (`self.CE_Destroy`)))

(event `self.Sphere.OnComponentBeginOverlap`
  (params (OverlappedComponent :type "PrimitiveComponent Object Reference") (OtherActor :type "Actor Object Reference") (OtherComp :type "PrimitiveComponent Object Reference") (OtherBodyIndex :type Integer) (bFromSweep :type Boolean) (SweepResult :type "HitResult Structure (by ref)"))
  (bind _outactors (`GameplayStatics.GetAllActorsOfClass` "/Game/BP/BP_ZiChen/BP_Hielo.BP_Hielo_C"))
  (if (== OtherActor (`|GetArrayItem` _outactors))
    (`self.EnableInput` (`GameplayStatics.GetPlayerController` 0))
    (`GameplayStatics.PlaySound2D` "/Game/Sounds/Dockable_Window_Pick_Up.Dockable_Window_Pick_Up" 1.0 1.0 0.0 null null :!label _label)))

(event `CE_Destroy`
  (`GameplayStatics.PlaySound2D` "/Game/Sounds/Leave_Simulate.Leave_Simulate" 1.0 1.0 0.0 null null)
  (`self.K2_DestroyActor`))

(event `self.Sphere.OnComponentEndOverlap`
  (params (OverlappedComponent :type "PrimitiveComponent Object Reference") (OtherActor :type "Actor Object Reference") (OtherComp :type "PrimitiveComponent Object Reference") (OtherBodyIndex :type Integer))
  (if (== OtherActor (`self.Player`))
    (`self.DisableInput` (`GameplayStatics.GetPlayerController` 0))
    (goto _label)))

(fn `UserConstructionScript`)