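; BP_FirebleIce is an actor with a box trigger and a Niagara effect that reacts to BP_Ice actors.
; It caches the player character on BeginPlay and loops over all BP_Ice actors every Tick with an empty body.
; Box overlap compares the other actor to that loop's element, effectively the last one found.
; On a match with player IceLevel1 or IceLevel2, it rescales the effect to half size and sets CanDistroyed.
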(event `self.ReceiveBeginPlay`
  (bind _asbp_top_down_character (cast `/Game/TopDown/Blueprints/BP_TopDownCharacter` (`GameplayStatics.GetPlayerCharacter` 0)))
  (set `self.player` _asbp_top_down_character))

(event `self.ReceiveTick`
  (params (DeltaSeconds :type "Float (single-precision)"))
  (bind _outactors (`GameplayStatics.GetAllActorsOfClass` "/Game/BP/BP_ZiChen/Magic/BP_Ice.BP_Ice_C"))
  (for _array_element _outactors
    _))

(event `self.Box.OnComponentBeginOverlap`
  (params (OverlappedComponent :type "PrimitiveComponent Object Reference") (OtherActor :type "Actor Object Reference") (OtherComp :type "PrimitiveComponent Object Reference") (OtherBodyIndex :type Integer) (bFromSweep :type Boolean) (SweepResult :type "HitResult Structure (by ref)"))
  (if (and (== (stale `self.ReceiveTick` _array_element) OtherActor) (or (`/Game/TopDown/Blueprints/BP_TopDownCharacter.IceLevel_1` (`self.player`)) (`/Game/TopDown/Blueprints/BP_TopDownCharacter.IceLevel_2` (`self.player`))))
    (`SceneComponent.SetRelativeScale3D` (`self.Niagara`) (0.5 0.5 0.5))
    (set `self.canDistroyed?` true)))

(fn `UserConstructionScript`)