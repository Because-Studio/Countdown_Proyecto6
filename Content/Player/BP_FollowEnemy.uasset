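; BP_FollowEnemy is an enemy that follows while an actor is inside its detection sphere, intended for the player.
; Sphere overlap begin sets FollowPlayer and starts a follow event that issues AI MoveTo and re-calls itself every 0.2 seconds.
; A distance check switches the move target to the enemy itself at close range.
; Overlap end checks the leaving actor, then clears the flag and stops movement immediately.
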(event `self.ReceiveBeginPlay`
  ;[1 1 1] Begin_Playe
)

(event `self.Sphere.OnComponentEndOverlap`
  (params (OverlappedComponent :type "PrimitiveComponent Object Reference") (OtherActor :type "Actor Object Reference") (OtherComp :type "PrimitiveComponent Object Reference") (OtherBodyIndex :type Integer))
  ;[1 1 1] Col_End
  (if (== OtherActor null)
    (set `self.FollowPlayer?` false)
    (`self.CE_StopMove`)
    (`KismetSystemLibrary.PrintString` "Player_Out")))

(event `self.Sphere.OnComponentBeginOverlap`
  (params (OverlappedComponent :type "PrimitiveComponent Object Reference") (OtherActor :type "Actor Object Reference") (OtherComp :type "PrimitiveComponent Object Reference") (OtherBodyIndex :type Integer) (bFromSweep :type Boolean) (SweepResult :type "HitResult Structure (by ref)"))
  ;[1 1 1] Col_Enter
  (set `self.FollowPlayer?` true)
  (`self.CE_FollowPlayer`)
  (`KismetSystemLibrary.PrintString` "Player_Enter"))

(event `CE_FollowPlayer`
  ;[1 1 1] Follow_Player
  (if (`self.FollowPlayer?`)
    (if (>= (`self.GetDistanceTo` null) 100.0)
      (`|AIMoveTo` self (0.0 0.0 0.0) null
        (:`then`
          _))
      (else
        (`|AIMoveTo` self (0.0 0.0 0.0) self
          (:`then`
            _))))
    (`KismetSystemLibrary.Delay` 0.2)
    (`self.CE_FollowPlayer`)))

(event `CE_StopMove`
  ;[1 1 1] CE_Stop_Move
  (set `self.FollowPlayer?` false)
  (`MovementComponent.StopMovementImmediately` (`self.CharacterMovement`)))

(fn `UserConstructionScript`)